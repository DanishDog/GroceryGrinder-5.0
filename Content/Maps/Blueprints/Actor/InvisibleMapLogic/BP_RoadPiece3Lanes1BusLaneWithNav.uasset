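; Invisible road piece actor that guides vehicles along three regular lanes and one bus lane.
; Each lane pairs a trigger box with its own spline.
; When a BP_Vehicle_Master overlaps a box, it receives that lane's spline as its current path, along with the piece's shared speed limit.
; Other overlapping actors fail the cast and are ignored.
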(event `self.Box1.OnComponentBeginOverlap`
  (params (OverlappedComponent :type "PrimitiveComponent Object Reference") (OtherActor :type "Actor Object Reference") (OtherComp :type "PrimitiveComponent Object Reference") (OtherBodyIndex :type Integer) (bFromSweep :type Boolean) (SweepResult :type "HitResult Structure (by ref)"))
  (bind _asbp_vehicle_master (cast `/Game/NPC/Vehicles/BP_Vehicle_Master` OtherActor)) ; Casting has 2 purposes here: \n1) check if the object that overlapped is a vehicle (to avoid e.g. a banana to drive - which would make cast fail and stop the logic) \nand 2) being able to call functions from the vehicle afterwards
  (set `/Game/NPC/Vehicles/BP_Vehicle_Master.CurrentPath` (`self.Spline1`) _asbp_vehicle_master)
  (set `/Game/NPC/Vehicles/BP_Vehicle_Master.CurrentStreetSpeedLimit` (`self.SpeedLimit`) _asbp_vehicle_master))

(event `self.Box2.OnComponentBeginOverlap`
  (params (OverlappedComponent :type "PrimitiveComponent Object Reference") (OtherActor :type "Actor Object Reference") (OtherComp :type "PrimitiveComponent Object Reference") (OtherBodyIndex :type Integer) (bFromSweep :type Boolean) (SweepResult :type "HitResult Structure (by ref)"))
  (bind _asbp_vehicle_master (cast `/Game/NPC/Vehicles/BP_Vehicle_Master` OtherActor))
  (set `/Game/NPC/Vehicles/BP_Vehicle_Master.CurrentPath` (`self.Spline2`) _asbp_vehicle_master)
  (set `/Game/NPC/Vehicles/BP_Vehicle_Master.CurrentStreetSpeedLimit` (`self.SpeedLimit`) _asbp_vehicle_master))

(event `self.Box3.OnComponentBeginOverlap`
  (params (OverlappedComponent :type "PrimitiveComponent Object Reference") (OtherActor :type "Actor Object Reference") (OtherComp :type "PrimitiveComponent Object Reference") (OtherBodyIndex :type Integer) (bFromSweep :type Boolean) (SweepResult :type "HitResult Structure (by ref)"))
  (bind _asbp_vehicle_master (cast `/Game/NPC/Vehicles/BP_Vehicle_Master` OtherActor))
  (set `/Game/NPC/Vehicles/BP_Vehicle_Master.CurrentPath` (`self.Spline3`) _asbp_vehicle_master)
  (set `/Game/NPC/Vehicles/BP_Vehicle_Master.CurrentStreetSpeedLimit` (`self.SpeedLimit`) _asbp_vehicle_master))

(event `self.BoxBus.OnComponentBeginOverlap`
  (params (OverlappedComponent :type "PrimitiveComponent Object Reference") (OtherActor :type "Actor Object Reference") (OtherComp :type "PrimitiveComponent Object Reference") (OtherBodyIndex :type Integer) (bFromSweep :type Boolean) (SweepResult :type "HitResult Structure (by ref)"))
  (bind _asbp_vehicle_master (cast `/Game/NPC/Vehicles/BP_Vehicle_Master` OtherActor))
  (set `/Game/NPC/Vehicles/BP_Vehicle_Master.CurrentPath` (`self.SplineBus`) _asbp_vehicle_master)
  (set `/Game/NPC/Vehicles/BP_Vehicle_Master.CurrentStreetSpeedLimit` (`self.SpeedLimit`) _asbp_vehicle_master))

(fn `UserConstructionScript`)