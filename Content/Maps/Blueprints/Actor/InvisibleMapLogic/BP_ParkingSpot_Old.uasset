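; Parking spot actor, marked old by name, that lets passing BP_Vehicle_Master cars claim, park in and leave a space.
; Left and right entry boxes randomly assign the free spot to park-seeking vehicles, passing side-specific entry and shared exit splines.
; Claims set IsOccupied immediately to avoid double booking.
; The spot box stops arriving vehicles and marks them parked; any overlapping actor occupies it, and any departure frees it.
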(event `self.ReceiveBeginPlay`
  (set `self.ParkingSpotLocationInWorld` (+ (`self.K2_GetActorLocation`) (200.0 250.0 50.0))))

(event `self.BoxEnterParkingSpotRight.OnComponentBeginOverlap`
  (params (OverlappedComponent :type "PrimitiveComponent Object Reference") (OtherActor :type "Actor Object Reference") (OtherComp :type "PrimitiveComponent Object Reference") (OtherBodyIndex :type Integer) (bFromSweep :type Boolean) (SweepResult :type "HitResult Structure (by ref)"))
  (if (not (`self.IsOccupied`))
    (bind _asbp_vehicle_master (cast `/Game/NPC/Vehicles/BP_Vehicle_Master` OtherActor))
    (if (`/Game/NPC/Vehicles/BP_Vehicle_Master.isGoingToPark` _asbp_vehicle_master)
      ;[1 1 1] randomizer - if parking spot available - still only take it 1 times out of 5 - to ensure full parking is used
      (if (== (`KismetMathLibrary.RandomIntegerInRange` 0 5) 5)
        (set `/Game/NPC/Vehicles/BP_Vehicle_Master.CurrentParkingSpot` self _asbp_vehicle_master)
        (set `/Game/NPC/Vehicles/BP_Vehicle_Master.ParkingSteeringPosition` (`self.SplineParkingPathRight`) _asbp_vehicle_master)
        (set `/Game/NPC/Vehicles/BP_Vehicle_Master.hasFoundParkingSpot` true _asbp_vehicle_master)
        (set `self.IsOccupied` true) ; here as well to be sure if 2 cars are very close to each other\nand the first has not finished parking yet (in which case the isoccupied\nwould still be false)
        (set `/Game/NPC/Vehicles/BP_Vehicle_Master.ParkingSpotExitPath` (`self.SplineParkingExit`) _asbp_vehicle_master)))))

(event `self.BoxEnterParkingSpotLeft.OnComponentBeginOverlap`
  (params (OverlappedComponent :type "PrimitiveComponent Object Reference") (OtherActor :type "Actor Object Reference") (OtherComp :type "PrimitiveComponent Object Reference") (OtherBodyIndex :type Integer) (bFromSweep :type Boolean) (SweepResult :type "HitResult Structure (by ref)"))
  (if (not (`self.IsOccupied`))
    (bind _asbp_vehicle_master (cast `/Game/NPC/Vehicles/BP_Vehicle_Master` OtherActor))
    (if (`/Game/NPC/Vehicles/BP_Vehicle_Master.isGoingToPark` _asbp_vehicle_master)
      ;[1 1 1] randomizer - if parking spot available - still only take it 1 times out of 5 - to ensure full parking is used
      (if (== (`KismetMathLibrary.RandomIntegerInRange` 0 5) 5)
        (set `/Game/NPC/Vehicles/BP_Vehicle_Master.CurrentParkingSpot` self _asbp_vehicle_master)
        (set `/Game/NPC/Vehicles/BP_Vehicle_Master.ParkingSteeringPosition` (`self.SplineParkingPathLeft`) _asbp_vehicle_master)
        (set `/Game/NPC/Vehicles/BP_Vehicle_Master.hasFoundParkingSpot` true _asbp_vehicle_master)
        (set `self.IsOccupied` true)
        (set `/Game/NPC/Vehicles/BP_Vehicle_Master.ParkingSpotExitPath` (`self.SplineParkingExit`) _asbp_vehicle_master)))))

(event `self.BoxParkingSpot.OnComponentBeginOverlap`
  (params (OverlappedComponent :type "PrimitiveComponent Object Reference") (OtherActor :type "Actor Object Reference") (OtherComp :type "PrimitiveComponent Object Reference") (OtherBodyIndex :type Integer) (bFromSweep :type Boolean) (SweepResult :type "HitResult Structure (by ref)"))
  (set `self.IsOccupied` true)
  (bind _asbp_vehicle_master (cast `/Game/NPC/Vehicles/BP_Vehicle_Master` OtherActor))
  (`/Game/NPC/Vehicles/BP_Vehicle_Master.Stop` _asbp_vehicle_master)
  (set `/Game/NPC/Vehicles/BP_Vehicle_Master.isParked` true _asbp_vehicle_master))

(event `self.BoxParkingSpot.OnComponentEndOverlap`
  (params (OverlappedComponent :type "PrimitiveComponent Object Reference") (OtherActor :type "Actor Object Reference") (OtherComp :type "PrimitiveComponent Object Reference") (OtherBodyIndex :type Integer))
  (set `self.IsOccupied` false) ; this come BEFORE the cast to vehicle step\nas if not a vehicle standing on parking spot and\nthat thing leaves (e.g. a person), we still want the parking\nto go back to non-occupied
  (bind _asbp_vehicle_master (cast `/Game/NPC/Vehicles/BP_Vehicle_Master` OtherActor))
  (set `/Game/NPC/Vehicles/BP_Vehicle_Master.isParked` false _asbp_vehicle_master))

(fn `UserConstructionScript`)