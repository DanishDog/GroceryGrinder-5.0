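; Invisible road-logic actor for a crossroad with parking access that steers vehicles along splines.
; Trigger boxes cast overlapping actors to BP_Vehicle_Master, then set their current path spline and street speed limit.
; Most boxes assign a fixed spline, while two junction boxes switch on the vehicle's destination, sending Supermarket Parking traffic into the parking turn and other listed destinations straight on.
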(event `self.Box1.OnComponentBeginOverlap`
  (params (OverlappedComponent :type "PrimitiveComponent Object Reference") (OtherActor :type "Actor Object Reference") (OtherComp :type "PrimitiveComponent Object Reference") (OtherBodyIndex :type Integer) (bFromSweep :type Boolean) (SweepResult :type "HitResult Structure (by ref)"))
  (bind _asbp_vehicle_master (cast `/Game/NPC/Vehicles/BP_Vehicle_Master` OtherActor)) ; Casting has 2 purposes here: \n1) check if the object that overlapped is a vehicle (to avoid e.g. a banana to drive - which would make cast fail and stop the logic) \nand 2) being able to call functions from the vehicle afterwards
  (set `/Game/NPC/Vehicles/BP_Vehicle_Master.CurrentPath` (`self.Spline1`) _asbp_vehicle_master)
  (set `/Game/NPC/Vehicles/BP_Vehicle_Master.CurrentStreetSpeedLimit` (`self.SpeedLimit`) _asbp_vehicle_master))

(event `self.Box2.OnComponentBeginOverlap`
  (params (OverlappedComponent :type "PrimitiveComponent Object Reference") (OtherActor :type "Actor Object Reference") (OtherComp :type "PrimitiveComponent Object Reference") (OtherBodyIndex :type Integer) (bFromSweep :type Boolean) (SweepResult :type "HitResult Structure (by ref)"))
  (bind _asbp_vehicle_master (cast `/Game/NPC/Vehicles/BP_Vehicle_Master` OtherActor))
  (set `/Game/NPC/Vehicles/BP_Vehicle_Master.CurrentPath` (`self.Spline2`) _asbp_vehicle_master)
  (set `/Game/NPC/Vehicles/BP_Vehicle_Master.CurrentStreetSpeedLimit` (`self.SpeedLimit`) _asbp_vehicle_master))

(event `self.Box3.OnComponentBeginOverlap`
  (params (OverlappedComponent :type "PrimitiveComponent Object Reference") (OtherActor :type "Actor Object Reference") (OtherComp :type "PrimitiveComponent Object Reference") (OtherBodyIndex :type Integer) (bFromSweep :type Boolean) (SweepResult :type "HitResult Structure (by ref)"))
  (bind _asbp_vehicle_master (cast `/Game/NPC/Vehicles/BP_Vehicle_Master` OtherActor))
  (set `/Game/NPC/Vehicles/BP_Vehicle_Master.CurrentPath` (`self.Spline3`) _asbp_vehicle_master)
  (set `/Game/NPC/Vehicles/BP_Vehicle_Master.CurrentStreetSpeedLimit` (`self.SpeedLimit`) _asbp_vehicle_master))

(event `self.Box4.OnComponentBeginOverlap`
  (params (OverlappedComponent :type "PrimitiveComponent Object Reference") (OtherActor :type "Actor Object Reference") (OtherComp :type "PrimitiveComponent Object Reference") (OtherBodyIndex :type Integer) (bFromSweep :type Boolean) (SweepResult :type "HitResult Structure (by ref)"))
  (bind _asbp_vehicle_master (cast `/Game/NPC/Vehicles/BP_Vehicle_Master` OtherActor))
  (set `/Game/NPC/Vehicles/BP_Vehicle_Master.CurrentPath` (`self.Spline4`) _asbp_vehicle_master)
  (set `/Game/NPC/Vehicles/BP_Vehicle_Master.CurrentStreetSpeedLimit` (`self.SpeedLimit`) _asbp_vehicle_master))

(event `self.Box9.OnComponentBeginOverlap`
  (params (OverlappedComponent :type "PrimitiveComponent Object Reference") (OtherActor :type "Actor Object Reference") (OtherComp :type "PrimitiveComponent Object Reference") (OtherBodyIndex :type Integer) (bFromSweep :type Boolean) (SweepResult :type "HitResult Structure (by ref)"))
  (bind _asbp_vehicle_master (cast `/Game/NPC/Vehicles/BP_Vehicle_Master` OtherActor))
  (set `/Game/NPC/Vehicles/BP_Vehicle_Master.CurrentPath` (`self.Spline9`) _asbp_vehicle_master)
  (set `/Game/NPC/Vehicles/BP_Vehicle_Master.CurrentStreetSpeedLimit` (`self.SpeedLimit`) _asbp_vehicle_master))

(event `self.Box12.OnComponentBeginOverlap`
  (params (OverlappedComponent :type "PrimitiveComponent Object Reference") (OtherActor :type "Actor Object Reference") (OtherComp :type "PrimitiveComponent Object Reference") (OtherBodyIndex :type Integer) (bFromSweep :type Boolean) (SweepResult :type "HitResult Structure (by ref)"))
  (bind _asbp_vehicle_master (cast `/Game/NPC/Vehicles/BP_Vehicle_Master` OtherActor))
  (set `/Game/NPC/Vehicles/BP_Vehicle_Master.CurrentPath` (`self.Spline12`) _asbp_vehicle_master)
  (set `/Game/NPC/Vehicles/BP_Vehicle_Master.CurrentStreetSpeedLimit` (`self.SpeedLimit`) _asbp_vehicle_master))

(event `self.Box10.OnComponentBeginOverlap`
  (params (OverlappedComponent :type "PrimitiveComponent Object Reference") (OtherActor :type "Actor Object Reference") (OtherComp :type "PrimitiveComponent Object Reference") (OtherBodyIndex :type Integer) (bFromSweep :type Boolean) (SweepResult :type "HitResult Structure (by ref)"))
  (bind _asbp_vehicle_master (cast `/Game/NPC/Vehicles/BP_Vehicle_Master` OtherActor))
  (set `/Game/NPC/Vehicles/BP_Vehicle_Master.CurrentStreetSpeedLimit` (`self.SpeedLimit`) _asbp_vehicle_master)
  (switch `/Game/NPC/Vehicles/VehicleDestinations` (`/Game/NPC/Vehicles/BP_Vehicle_Master.CurrentDestination` _asbp_vehicle_master) ; choose the next spline to drive to based on the current position and the destination
    (:`NewEnumerator0`
      (set `/Game/NPC/Vehicles/BP_Vehicle_Master.CurrentPath` (`self.TopRightGoParking`) _asbp_vehicle_master))
    (:`NewEnumerator1`
      (set `/Game/NPC/Vehicles/BP_Vehicle_Master.CurrentPath` (`self.TopRightGoStraight`) _asbp_vehicle_master :!label _label))
    (:`NewEnumerator2`
      (goto _label))
    (:`NewEnumerator3`
      (goto _label))
    (:`NewEnumerator4`
      (goto _label))))

(event `self.Box6.OnComponentBeginOverlap`
  (params (OverlappedComponent :type "PrimitiveComponent Object Reference") (OtherActor :type "Actor Object Reference") (OtherComp :type "PrimitiveComponent Object Reference") (OtherBodyIndex :type Integer) (bFromSweep :type Boolean) (SweepResult :type "HitResult Structure (by ref)"))
  (bind _asbp_vehicle_master (cast `/Game/NPC/Vehicles/BP_Vehicle_Master` OtherActor))
  (set `/Game/NPC/Vehicles/BP_Vehicle_Master.CurrentStreetSpeedLimit` (`self.SpeedLimit`) _asbp_vehicle_master)
  (switch `/Game/NPC/Vehicles/VehicleDestinations` (`/Game/NPC/Vehicles/BP_Vehicle_Master.CurrentDestination` _asbp_vehicle_master) ; choose the next spline to drive to based on the current position and the destination
    (:`NewEnumerator0`
      (set `/Game/NPC/Vehicles/BP_Vehicle_Master.CurrentPath` (`self.MiddleLeftGoParking`) _asbp_vehicle_master))
    (:`NewEnumerator1`
      (set `/Game/NPC/Vehicles/BP_Vehicle_Master.CurrentPath` (`self.MiddleLeftGoStraight`) _asbp_vehicle_master :!label _label_2))
    (:`NewEnumerator2`
      (goto _label_2))
    (:`NewEnumerator3`
      (goto _label_2))
    (:`NewEnumerator4`
      (goto _label_2))))

(fn `UserConstructionScript`)