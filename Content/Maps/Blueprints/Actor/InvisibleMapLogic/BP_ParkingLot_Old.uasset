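; BP_ParkingLot_Old is a map logic actor that routes vehicles entering a parking lot.
; When a BP_Vehicle_Master overlaps ParkingEntry, a weighted random pick assigns one of three entry routes, favouring two with 3-in-7 odds each.
; It also sets the vehicle's route ID and speed limit, plus a lot reference for exit-route lookup.
; Route IDs are crossed: Entry2 records 3 and Entry3 records 2.
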(event `self.ParkingEntry.OnComponentBeginOverlap`
  (params (OverlappedComponent :type "PrimitiveComponent Object Reference") (OtherActor :type "Actor Object Reference") (OtherComp :type "PrimitiveComponent Object Reference") (OtherBodyIndex :type Integer) (bFromSweep :type Boolean) (SweepResult :type "HitResult Structure (by ref)"))
  (bind _asbp_vehicle_master (cast `/Game/NPC/Vehicles/BP_Vehicle_Master` OtherActor))
  (switch `int` (`KismetMathLibrary.RandomIntegerInRange` 0 6) ; random selection of parking route - \nbut "weighed" because some routes \nhave much more spaces
    (:`0`
      (set `/Game/NPC/Vehicles/BP_Vehicle_Master.CurrentPath` (`self.ParkingRouteEntry1`) _asbp_vehicle_master :!label _label)
      (set `/Game/NPC/Vehicles/BP_Vehicle_Master.ParkingRouteTaken` 1 _asbp_vehicle_master))
    (:`1`
      (goto _label))
    (:`2`
      (goto _label))
    (:`3`
      (set `/Game/NPC/Vehicles/BP_Vehicle_Master.CurrentPath` (`self.ParkingRouteEntry2`) _asbp_vehicle_master :!label _label_2)
      (set `/Game/NPC/Vehicles/BP_Vehicle_Master.ParkingRouteTaken` 3 _asbp_vehicle_master))
    (:`4`
      (goto _label_2))
    (:`5`
      (goto _label_2))
    (:`6`
      (set `/Game/NPC/Vehicles/BP_Vehicle_Master.CurrentPath` (`self.ParkingRouteEntry3`) _asbp_vehicle_master)
      (set `/Game/NPC/Vehicles/BP_Vehicle_Master.ParkingRouteTaken` 2 _asbp_vehicle_master)))
  (set `/Game/NPC/Vehicles/BP_Vehicle_Master.CurrentStreetSpeedLimit` (`self.Speedlimit`) _asbp_vehicle_master)
  (set `/Game/NPC/Vehicles/BP_Vehicle_Master.ParkingLot` self _asbp_vehicle_master) ; used for referencing the exitroutes easily in the vehicle class
)

(fn `UserConstructionScript`)