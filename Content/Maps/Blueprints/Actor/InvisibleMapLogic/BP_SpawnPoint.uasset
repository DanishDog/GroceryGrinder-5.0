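; BP_SpawnPoint is an invisible map actor that feeds AI vehicles into traffic from its own location and rotation.
; It spawns a BP_Vehicle_Master on BeginPlay, then loops every 30 seconds, spawning again while MapCounter reports ten or fewer cars.
; Each vehicle receives StartingPath and an explicit Drive call, because construction-time driving runs before the path is set, then increments the shared count.
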(event `self.ReceiveBeginPlay`
  (`self.Spawn`)
  ;[1 1 1] spawn new car every 30 seconds if total number of cars on map is still smaller than or equal to ...
  (if (<= (`/Game/Maps/Blueprints/Actor/InvisibleMapLogic/BP_MapCounter.NumberOfCarsInMap` (`self.MapCounter`)) 10) :!label _label
    (`KismetSystemLibrary.RetriggerableDelay` 30.0)
    (`self.Spawn`)
    (goto _label)
    (else
      (`KismetSystemLibrary.RetriggerableDelay` 30.0)
      (goto _label))))

(fn `Spawn`
  (bind (_returnvalue_location _returnvalue_rotation) (`KismetMathLibrary.BreakTransform` (`self.GetTransform` self)))
  (bind _returnvalue (`AIBlueprintHelperLibrary.SpawnAIFromClass` "/Game/NPC/Vehicles/BP_Vehicle_Master.BP_Vehicle_Master_C" null _returnvalue_location _returnvalue_rotation false null)) ; this will call the construction script of the bp vehicle master class
  (set `self.Spawned` true)
  (bind _asbp_vehicle_master (cast `/Game/NPC/Vehicles/BP_Vehicle_Master` _returnvalue))
  (set `/Game/NPC/Vehicles/BP_Vehicle_Master.CurrentPath` (`self.StartingPath`) _asbp_vehicle_master)
  (`/Game/NPC/Vehicles/BP_Vehicle_Master.Drive` _asbp_vehicle_master) ; needed here explicitely - because the "drive" call\npart of the constructor of the bp-vehicle is called BEFORE\nthe set path to starting path step. Otherwise car does not move\nforward
  (`/Game/Maps/Blueprints/Actor/InvisibleMapLogic/BP_MapCounter.IncreaseNumberOfCarsInMapWithOne` (`self.MapCounter`)))

(fn `UserConstructionScript`)