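; Crossroad road piece that steers BP_Vehicle_Master vehicles through the junction by setting their CurrentPath to splines when they overlap trigger boxes.
; Entry, exit and bus boxes assign fixed splines, while decision boxes pick one from the vehicle's CurrentDestination, sometimes choosing a lane at random.
; Speed boxes slow vehicles on approach so they stay on the splines, then restore default speed on exit.
; Return and lane-switch routes are temporary stand-ins.
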(event `self.Box2.OnComponentBeginOverlap`
  (params (OverlappedComponent :type "PrimitiveComponent Object Reference") (OtherActor :type "Actor Object Reference") (OtherComp :type "PrimitiveComponent Object Reference") (OtherBodyIndex :type Integer) (bFromSweep :type Boolean) (SweepResult :type "HitResult Structure (by ref)"))
  ;[1 1 1] Simple logic to enter and leave the cross road - excluding the points where a decision is needed
  (bind _asbp_vehicle_master (cast `/Game/NPC/Vehicles/BP_Vehicle_Master` OtherActor))
  (set `/Game/NPC/Vehicles/BP_Vehicle_Master.CurrentPath` (`self.Spline2`) _asbp_vehicle_master))

(event `self.Box3.OnComponentBeginOverlap`
  (params (OverlappedComponent :type "PrimitiveComponent Object Reference") (OtherActor :type "Actor Object Reference") (OtherComp :type "PrimitiveComponent Object Reference") (OtherBodyIndex :type Integer) (bFromSweep :type Boolean) (SweepResult :type "HitResult Structure (by ref)"))
  ;[1 1 1] Simple logic to enter and leave the cross road - excluding the points where a decision is needed
  (bind _asbp_vehicle_master (cast `/Game/NPC/Vehicles/BP_Vehicle_Master` OtherActor))
  (set `/Game/NPC/Vehicles/BP_Vehicle_Master.CurrentPath` (`self.Spline3`) _asbp_vehicle_master))

(event `self.Box6.OnComponentBeginOverlap`
  (params (OverlappedComponent :type "PrimitiveComponent Object Reference") (OtherActor :type "Actor Object Reference") (OtherComp :type "PrimitiveComponent Object Reference") (OtherBodyIndex :type Integer) (bFromSweep :type Boolean) (SweepResult :type "HitResult Structure (by ref)"))
  ;[1 1 1] Simple logic to enter and leave the cross road - excluding the points where a decision is needed
  (bind _asbp_vehicle_master (cast `/Game/NPC/Vehicles/BP_Vehicle_Master` OtherActor))
  (set `/Game/NPC/Vehicles/BP_Vehicle_Master.CurrentPath` (`self.Spline6`) _asbp_vehicle_master))

(event `self.Box4.OnComponentBeginOverlap`
  (params (OverlappedComponent :type "PrimitiveComponent Object Reference") (OtherActor :type "Actor Object Reference") (OtherComp :type "PrimitiveComponent Object Reference") (OtherBodyIndex :type Integer) (bFromSweep :type Boolean) (SweepResult :type "HitResult Structure (by ref)"))
  ;[1 1 1] Simple logic to enter and leave the cross road - excluding the points where a decision is needed
  (bind _asbp_vehicle_master (cast `/Game/NPC/Vehicles/BP_Vehicle_Master` OtherActor))
  (set `/Game/NPC/Vehicles/BP_Vehicle_Master.CurrentPath` (`self.Spline4`) _asbp_vehicle_master))

(event `self.BoxBus.OnComponentBeginOverlap`
  (params (OverlappedComponent :type "PrimitiveComponent Object Reference") (OtherActor :type "Actor Object Reference") (OtherComp :type "PrimitiveComponent Object Reference") (OtherBodyIndex :type Integer) (bFromSweep :type Boolean) (SweepResult :type "HitResult Structure (by ref)"))
  ;[1 1 1] Simple logic to enter and leave the cross road - excluding the points where a decision is needed
  (bind _asbp_vehicle_master (cast `/Game/NPC/Vehicles/BP_Vehicle_Master` OtherActor))
  (set `/Game/NPC/Vehicles/BP_Vehicle_Master.CurrentPath` (`self.SplineBus`) _asbp_vehicle_master))

(event `self.BoxBus1.OnComponentBeginOverlap`
  (params (OverlappedComponent :type "PrimitiveComponent Object Reference") (OtherActor :type "Actor Object Reference") (OtherComp :type "PrimitiveComponent Object Reference") (OtherBodyIndex :type Integer) (bFromSweep :type Boolean) (SweepResult :type "HitResult Structure (by ref)"))
  ;[1 1 1] Simple logic to enter and leave the cross road - excluding the points where a decision is needed
  (bind _asbp_vehicle_master (cast `/Game/NPC/Vehicles/BP_Vehicle_Master` OtherActor))
  (set `/Game/NPC/Vehicles/BP_Vehicle_Master.CurrentPath` (`self.SplineBusCrossRoad`) _asbp_vehicle_master))

(event `self.Box7.OnComponentBeginOverlap`
  (params (OverlappedComponent :type "PrimitiveComponent Object Reference") (OtherActor :type "Actor Object Reference") (OtherComp :type "PrimitiveComponent Object Reference") (OtherBodyIndex :type Integer) (bFromSweep :type Boolean) (SweepResult :type "HitResult Structure (by ref)"))
  ;[1 1 1] Simple logic to enter and leave the cross road - excluding the points where a decision is needed
  (bind _asbp_vehicle_master (cast `/Game/NPC/Vehicles/BP_Vehicle_Master` OtherActor))
  (set `/Game/NPC/Vehicles/BP_Vehicle_Master.CurrentPath` (`self.Spline7`) _asbp_vehicle_master))

(event `self.DecisionBoxLeftMiddle.OnComponentBeginOverlap`
  (params (OverlappedComponent :type "PrimitiveComponent Object Reference") (OtherActor :type "Actor Object Reference") (OtherComp :type "PrimitiveComponent Object Reference") (OtherBodyIndex :type Integer) (bFromSweep :type Boolean) (SweepResult :type "HitResult Structure (by ref)"))
  ;[1 1 1] Cross road decision logic - based on the current position of the car (= the decisionBox it overlaps with) and the current destination of the car -> combination leads to the selection of a destination box (and spline) to drive to
  (bind _asbp_vehicle_master (cast `/Game/NPC/Vehicles/BP_Vehicle_Master` OtherActor)) ; Casting has 2 purposes here: \n1) check if the object that overlapped is a vehicle (to avoid e.g. a banana to drive - which would make cast fail and stop the logic) \nand 2) being able to call functions from the vehicle afterwards
  (switch `/Game/NPC/Vehicles/VehicleDestinations` (`/Game/NPC/Vehicles/BP_Vehicle_Master.CurrentDestination` _asbp_vehicle_master) ; choose the next spline to drive to based on the current position and the destination
    (:`NewEnumerator0`
      (set `/Game/NPC/Vehicles/BP_Vehicle_Master.CurrentPath` (`self.LeftMiddleToTopRight`) _asbp_vehicle_master :!label _label) ; Turn back left
    )
    (:`NewEnumerator1`
      ;;[1 1 1] To go "upwards" on the road on the right, there is 2 lanes - this picks 1 of the 2 randomly
      (if (== (`KismetMathLibrary.RandomIntegerInRange` 0 1) 0) :!label _label_2
        (set `/Game/NPC/Vehicles/BP_Vehicle_Master.CurrentPath` (`self.LeftMiddleToTopMiddle`) _asbp_vehicle_master) ; Go up on middle lane
        (else
          (set `/Game/NPC/Vehicles/BP_Vehicle_Master.CurrentPath` (`self.LeftMiddleToTopRight`) _asbp_vehicle_master) ; Go up on right lane
        )))
    (:`NewEnumerator2`
      (goto _label))
    (:`NewEnumerator3`
      (set `/Game/NPC/Vehicles/BP_Vehicle_Master.CurrentPath` (`self.LeftMiddleToBottomLeft`) _asbp_vehicle_master) ; Go down
    )
    (:`NewEnumerator4`
      (goto _label_2))))

(event `self.DecisionBoxLeftBottom.OnComponentBeginOverlap`
  (params (OverlappedComponent :type "PrimitiveComponent Object Reference") (OtherActor :type "Actor Object Reference") (OtherComp :type "PrimitiveComponent Object Reference") (OtherBodyIndex :type Integer) (bFromSweep :type Boolean) (SweepResult :type "HitResult Structure (by ref)"))
  ;[1 1 1] Cross road decision logic - based on the current position of the car (= the decisionBox it overlaps with) and the current destination of the car -> combination leads to the selection of a destination box (and spline) to drive to
  (bind _asbp_vehicle_master (cast `/Game/NPC/Vehicles/BP_Vehicle_Master` OtherActor))
  (switch `/Game/NPC/Vehicles/VehicleDestinations` (`/Game/NPC/Vehicles/BP_Vehicle_Master.CurrentDestination` _asbp_vehicle_master) ; choose the next spline to drive to based on\n the current position and the destination
    (:`NewEnumerator0`
      (set `/Game/NPC/Vehicles/BP_Vehicle_Master.CurrentPath` (`self.LeftBottomToTopRight`) _asbp_vehicle_master :!label _label_3) ; Turn back left
    )
    (:`NewEnumerator1`
      ;;[1 1 1] To go "upwards" on the road on the right, there is 2 lanes - this picks 1 of the 2 randomly
      (if (== (`KismetMathLibrary.RandomIntegerInRange` 0 1) 0) :!label _label_4
        (set `/Game/NPC/Vehicles/BP_Vehicle_Master.CurrentPath` (`self.LeftBottomToTopMiddle`) _asbp_vehicle_master) ; Go up on middle lane
        (else
          (set `/Game/NPC/Vehicles/BP_Vehicle_Master.CurrentPath` (`self.LeftBottomToTopRight`) _asbp_vehicle_master) ; Go up on right lane
        )))
    (:`NewEnumerator2`
      (goto _label_3))
    (:`NewEnumerator3`
      (set `/Game/NPC/Vehicles/BP_Vehicle_Master.CurrentPath` (`self.LeftBottomToBottomLeft`) _asbp_vehicle_master) ; Go down
    )
    (:`NewEnumerator4`
      (goto _label_4))))

(event `self.DecisionBoxBottomMiddle.OnComponentBeginOverlap`
  (params (OverlappedComponent :type "PrimitiveComponent Object Reference") (OtherActor :type "Actor Object Reference") (OtherComp :type "PrimitiveComponent Object Reference") (OtherBodyIndex :type Integer) (bFromSweep :type Boolean) (SweepResult :type "HitResult Structure (by ref)"))
  ;[1 1 1] Cross road decision logic - based on the current position of the car (= the decisionBox it overlaps with) and the current destination of the car -> combination leads to the selection of a destination box (and spline) to drive to
  (bind _asbp_vehicle_master (cast `/Game/NPC/Vehicles/BP_Vehicle_Master` OtherActor))
  (switch `/Game/NPC/Vehicles/VehicleDestinations` (`/Game/NPC/Vehicles/BP_Vehicle_Master.CurrentDestination` _asbp_vehicle_master) ; choose the next spline to drive to based on the current position and the destination
    (:`NewEnumerator0`
      (set `/Game/NPC/Vehicles/BP_Vehicle_Master.CurrentPath` (`self.BottomMiddleToLeftTop`) _asbp_vehicle_master :!label _label_5) ; Turn left
    )
    (:`NewEnumerator1`
      ;;[1 1 1] To go "upwards" on the road on the right, there is 2 lanes - this picks 1 of the 2 randomly
      (if (== (`KismetMathLibrary.RandomIntegerInRange` 0 1) 0) :!label _label_6
        (set `/Game/NPC/Vehicles/BP_Vehicle_Master.CurrentPath` (`self.BottomMiddleToTopMiddle`) _asbp_vehicle_master) ; Go up on middle lane
        (else
          (set `/Game/NPC/Vehicles/BP_Vehicle_Master.CurrentPath` (`self.BottomMiddleToTopMiddle`) _asbp_vehicle_master) ; Go up on right lane
        )))
    (:`NewEnumerator2`
      (goto _label_5))
    (:`NewEnumerator3`
      (set `/Game/NPC/Vehicles/BP_Vehicle_Master.CurrentPath` (`self.BottomMiddleToLeftTop`) _asbp_vehicle_master) ; Turn back down
    )
    (:`NewEnumerator4`
      (goto _label_6))))

(event `self.DecisionBoxBottomRight.OnComponentBeginOverlap`
  (params (OverlappedComponent :type "PrimitiveComponent Object Reference") (OtherActor :type "Actor Object Reference") (OtherComp :type "PrimitiveComponent Object Reference") (OtherBodyIndex :type Integer) (bFromSweep :type Boolean) (SweepResult :type "HitResult Structure (by ref)"))
  ;[1 1 1] Cross road decision logic - based on the current position of the car (= the decisionBox it overlaps with) and the current destination of the car -> combination leads to the selection of a destination box (and spline) to drive to
  (bind _asbp_vehicle_master (cast `/Game/NPC/Vehicles/BP_Vehicle_Master` OtherActor))
  (switch `/Game/NPC/Vehicles/VehicleDestinations` (`/Game/NPC/Vehicles/BP_Vehicle_Master.CurrentDestination` _asbp_vehicle_master) ; choose the next spline to drive to based on the current position and the destination
    (:`NewEnumerator0`
      (set `/Game/NPC/Vehicles/BP_Vehicle_Master.CurrentPath` (`self.BottomRightToLeftTop`) _asbp_vehicle_master :!label _label_7) ; Turn left
    )
    (:`NewEnumerator1`
      ;;[1 1 1] To go "upwards" on the road on the right, there is 2 lanes - this picks 1 of the 2 randomly
      (if (== (`KismetMathLibrary.RandomIntegerInRange` 0 1) 0) :!label _label_8
        (set `/Game/NPC/Vehicles/BP_Vehicle_Master.CurrentPath` (`self.BottomRightToTopRight`) _asbp_vehicle_master) ; Go up on middle lane
        (else
          (set `/Game/NPC/Vehicles/BP_Vehicle_Master.CurrentPath` (`self.BottomRightToTopRight`) _asbp_vehicle_master) ; Go up on right lane
        )))
    (:`NewEnumerator2`
      (goto _label_7))
    (:`NewEnumerator3`
      (set `/Game/NPC/Vehicles/BP_Vehicle_Master.CurrentPath` (`self.BottomRightToLeftTop`) _asbp_vehicle_master) ; Turn back down
    )
    (:`NewEnumerator4`
      (goto _label_8))))

(event `self.DecisionBoxTopLeft.OnComponentBeginOverlap`
  (params (OverlappedComponent :type "PrimitiveComponent Object Reference") (OtherActor :type "Actor Object Reference") (OtherComp :type "PrimitiveComponent Object Reference") (OtherBodyIndex :type Integer) (bFromSweep :type Boolean) (SweepResult :type "HitResult Structure (by ref)"))
  ;[1 1 1] Cross road decision logic - based on the current position of the car (= the decisionBox it overlaps with) and the current destination of the car -> combination leads to the selection of a destination box (and spline) to drive to
  (bind _asbp_vehicle_master (cast `/Game/NPC/Vehicles/BP_Vehicle_Master` OtherActor))
  (switch `/Game/NPC/Vehicles/VehicleDestinations` (`/Game/NPC/Vehicles/BP_Vehicle_Master.CurrentDestination` _asbp_vehicle_master) ; choose the next spline to drive to based on the current position and the destination
    (:`NewEnumerator0`
      (set `/Game/NPC/Vehicles/BP_Vehicle_Master.CurrentPath` (`self.TopLeftToLeftTop`) _asbp_vehicle_master :!label _label_9) ; Turn right
    )
    (:`NewEnumerator1`
      ;;[1 1 1] To go "upwards" on the road on the right, there is 2 lanes - this picks 1 of the 2 randomly
      (if (== (`KismetMathLibrary.RandomIntegerInRange` 0 1) 0) :!label _label_10
        (set `/Game/NPC/Vehicles/BP_Vehicle_Master.CurrentPath` (`self.TopLeftToLeftTop`) _asbp_vehicle_master) ; Go back up on middle lane
        (else
          (set `/Game/NPC/Vehicles/BP_Vehicle_Master.CurrentPath` (`self.TopLeftToBottomLeft`) _asbp_vehicle_master) ; Go back up on right lane
        )))
    (:`NewEnumerator2`
      (goto _label_9))
    (:`NewEnumerator3`
      (set `/Game/NPC/Vehicles/BP_Vehicle_Master.CurrentPath` (`self.TopLeftToBottomLeft`) _asbp_vehicle_master) ; Go down
    )
    (:`NewEnumerator4`
      (goto _label_10))))

(event `self.ResetSpeedTop.OnComponentBeginOverlap`
  (params (OverlappedComponent :type "PrimitiveComponent Object Reference") (OtherActor :type "Actor Object Reference") (OtherComp :type "PrimitiveComponent Object Reference") (OtherBodyIndex :type Integer) (bFromSweep :type Boolean) (SweepResult :type "HitResult Structure (by ref)"))
  ;[1 1 1] Slow down logic on cross road and reset speed when leaving crossroad - important to make the cars follow the spline paths (if too fast, they will deviate)
  (bind _asbp_vehicle_master (cast `/Game/NPC/Vehicles/BP_Vehicle_Master` OtherActor))
  (`/Game/NPC/Vehicles/BP_Vehicle_Master.SetMaxSpeedToDefaultMaxSpeed` _asbp_vehicle_master))

(event `self.ReduceSpeedTop.OnComponentBeginOverlap`
  (params (OverlappedComponent :type "PrimitiveComponent Object Reference") (OtherActor :type "Actor Object Reference") (OtherComp :type "PrimitiveComponent Object Reference") (OtherBodyIndex :type Integer) (bFromSweep :type Boolean) (SweepResult :type "HitResult Structure (by ref)"))
  ;[1 1 1] Slow down logic on cross road and reset speed when leaving crossroad - important to make the cars follow the spline paths (if too fast, they will deviate)
  (bind _asbp_vehicle_master (cast `/Game/NPC/Vehicles/BP_Vehicle_Master` OtherActor))
  (`/Game/NPC/Vehicles/BP_Vehicle_Master.Stop` _asbp_vehicle_master)
  (set `/Game/NPC/Vehicles/BP_Vehicle_Master.MaxSpeed` (`self.ReducedSpeedOnCrossRoad`) _asbp_vehicle_master)
  (`/Game/NPC/Vehicles/BP_Vehicle_Master.Drive` _asbp_vehicle_master))

(event `self.ReduceSpeedBottom.OnComponentBeginOverlap`
  (params (OverlappedComponent :type "PrimitiveComponent Object Reference") (OtherActor :type "Actor Object Reference") (OtherComp :type "PrimitiveComponent Object Reference") (OtherBodyIndex :type Integer) (bFromSweep :type Boolean) (SweepResult :type "HitResult Structure (by ref)"))
  ;[1 1 1] Slow down logic on cross road and reset speed when leaving crossroad - important to make the cars follow the spline paths (if too fast, they will deviate)
  (bind _asbp_vehicle_master (cast `/Game/NPC/Vehicles/BP_Vehicle_Master` OtherActor))
  (`/Game/NPC/Vehicles/BP_Vehicle_Master.Stop` _asbp_vehicle_master)
  (set `/Game/NPC/Vehicles/BP_Vehicle_Master.MaxSpeed` (`self.ReducedSpeedOnCrossRoad`) _asbp_vehicle_master)
  (`/Game/NPC/Vehicles/BP_Vehicle_Master.Drive` _asbp_vehicle_master))

(event `self.ResetSpeedBottom.OnComponentBeginOverlap`
  (params (OverlappedComponent :type "PrimitiveComponent Object Reference") (OtherActor :type "Actor Object Reference") (OtherComp :type "PrimitiveComponent Object Reference") (OtherBodyIndex :type Integer) (bFromSweep :type Boolean) (SweepResult :type "HitResult Structure (by ref)"))
  ;[1 1 1] Slow down logic on cross road and reset speed when leaving crossroad - important to make the cars follow the spline paths (if too fast, they will deviate)
  (bind _asbp_vehicle_master (cast `/Game/NPC/Vehicles/BP_Vehicle_Master` OtherActor))
  (`/Game/NPC/Vehicles/BP_Vehicle_Master.SetMaxSpeedToDefaultMaxSpeed` _asbp_vehicle_master))

(event `self.ReduceSpeedLeft.OnComponentBeginOverlap`
  (params (OverlappedComponent :type "PrimitiveComponent Object Reference") (OtherActor :type "Actor Object Reference") (OtherComp :type "PrimitiveComponent Object Reference") (OtherBodyIndex :type Integer) (bFromSweep :type Boolean) (SweepResult :type "HitResult Structure (by ref)"))
  ;[1 1 1] Slow down logic on cross road and reset speed when leaving crossroad - important to make the cars follow the spline paths (if too fast, they will deviate)
  (bind _asbp_vehicle_master (cast `/Game/NPC/Vehicles/BP_Vehicle_Master` OtherActor))
  (`/Game/NPC/Vehicles/BP_Vehicle_Master.Stop` _asbp_vehicle_master)
  (set `/Game/NPC/Vehicles/BP_Vehicle_Master.MaxSpeed` (`self.ReducedSpeedOnCrossRoad`) _asbp_vehicle_master)
  (`/Game/NPC/Vehicles/BP_Vehicle_Master.Drive` _asbp_vehicle_master))

(event `self.ResetSpeedLeft.OnComponentBeginOverlap`
  (params (OverlappedComponent :type "PrimitiveComponent Object Reference") (OtherActor :type "Actor Object Reference") (OtherComp :type "PrimitiveComponent Object Reference") (OtherBodyIndex :type Integer) (bFromSweep :type Boolean) (SweepResult :type "HitResult Structure (by ref)"))
  ;[1 1 1] Slow down logic on cross road and reset speed when leaving crossroad - important to make the cars follow the spline paths (if too fast, they will deviate)
  (bind _asbp_vehicle_master (cast `/Game/NPC/Vehicles/BP_Vehicle_Master` OtherActor))
  (`/Game/NPC/Vehicles/BP_Vehicle_Master.SetMaxSpeedToDefaultMaxSpeed` _asbp_vehicle_master))

(fn `UserConstructionScript`)