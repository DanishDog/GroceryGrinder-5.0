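; BP_ParkingSpot is a map logic actor that guides BP_Vehicle_Master vehicles into a parking spot.
; While the spot is free, left and right entry boxes assign it and the matching spline path to entering vehicles, flagging them to park.
; The spot box marks it occupied on any overlap, stops overlapping vehicles and clears occupancy on end overlap.
; BeginPlay caches an offset world location for the spot.
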(event `self.ReceiveBeginPlay`
  (set `self.ParkingSpotLocationInWorld` (+ (`self.K2_GetActorLocation`) (200.0 250.0 50.0))))

(event `self.BoxEnterParkingSpotRight.OnComponentBeginOverlap`
  (params (OverlappedComponent :type "PrimitiveComponent Object Reference") (OtherActor :type "Actor Object Reference") (OtherComp :type "PrimitiveComponent Object Reference") (OtherBodyIndex :type Integer) (bFromSweep :type Boolean) (SweepResult :type "HitResult Structure (by ref)"))
  (if (not (`self.IsOccupied`))
    (bind _asbp_vehicle_master (cast `/Game/NPC/Vehicles/BP_Vehicle_Master` OtherActor))
    (set `/Game/NPC/Vehicles/BP_Vehicle_Master.CurrentParkingSpot` self _asbp_vehicle_master)
    (set `/Game/NPC/Vehicles/BP_Vehicle_Master.ParkingSteeringPosition` (`self.SplineParkingPathRight`) _asbp_vehicle_master)
    (set `/Game/NPC/Vehicles/BP_Vehicle_Master.isGoingToPark` true _asbp_vehicle_master)
    (set `/Game/NPC/Vehicles/BP_Vehicle_Master.hasFoundParkingSpot` true _asbp_vehicle_master)))

(event `self.BoxEnterParkingSpotLeft.OnComponentBeginOverlap`
  (params (OverlappedComponent :type "PrimitiveComponent Object Reference") (OtherActor :type "Actor Object Reference") (OtherComp :type "PrimitiveComponent Object Reference") (OtherBodyIndex :type Integer) (bFromSweep :type Boolean) (SweepResult :type "HitResult Structure (by ref)"))
  (if (not (`self.IsOccupied`))
    (bind _asbp_vehicle_master (cast `/Game/NPC/Vehicles/BP_Vehicle_Master` OtherActor))
    (set `/Game/NPC/Vehicles/BP_Vehicle_Master.CurrentParkingSpot` self _asbp_vehicle_master)
    (set `/Game/NPC/Vehicles/BP_Vehicle_Master.ParkingSteeringPosition` (`self.SplineParkingPathLeft`) _asbp_vehicle_master)
    (set `/Game/NPC/Vehicles/BP_Vehicle_Master.isGoingToPark` true _asbp_vehicle_master)
    (set `/Game/NPC/Vehicles/BP_Vehicle_Master.hasFoundParkingSpot` true _asbp_vehicle_master)))

(event `self.BoxParkingSpot.OnComponentBeginOverlap`
  (params (OverlappedComponent :type "PrimitiveComponent Object Reference") (OtherActor :type "Actor Object Reference") (OtherComp :type "PrimitiveComponent Object Reference") (OtherBodyIndex :type Integer) (bFromSweep :type Boolean) (SweepResult :type "HitResult Structure (by ref)"))
  (set `self.IsOccupied` true)
  (bind _asbp_vehicle_master (cast `/Game/NPC/Vehicles/BP_Vehicle_Master` OtherActor))
  (`/Game/NPC/Vehicles/BP_Vehicle_Master.Stop` _asbp_vehicle_master))

(event `self.BoxParkingSpot.OnComponentEndOverlap`
  (params (OverlappedComponent :type "PrimitiveComponent Object Reference") (OtherActor :type "Actor Object Reference") (OtherComp :type "PrimitiveComponent Object Reference") (OtherBodyIndex :type Integer))
  (set `self.IsOccupied` false))

(fn `UserConstructionScript`)