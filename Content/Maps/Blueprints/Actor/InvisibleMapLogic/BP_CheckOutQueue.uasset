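; BP_CheckOutQueue is an invisible map-logic Blueprint that tracks occupancy of a three-spot checkout queue.
; Begin and end overlap events on the three queue location actors toggle per-spot occupied flags and update IsQueueFull.
; GetNextFreeQueueLocation returns the free spot nearest the checkout, assuming the caller has already confirmed the queue is not full.
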(event `self.QueueLocation1CheckOut.OnActorBeginOverlap`
  (params (OverlappedActor :type "Actor Object Reference") (OtherActor :type "Actor Object Reference"))
  (set `self.QueueLocation1Occupied` true)
  (`self.CheckAndSetQueueFullIndication` :!label _label))

(event `self.QueueLocation1CheckOut.OnActorEndOverlap`
  (params (OverlappedActor :type "Actor Object Reference") (OtherActor :type "Actor Object Reference"))
  (set `self.QueueLocation1Occupied` false)
  (set `self.IsQueueFull` false :!label _label_2))

(event `self.QueueLocation2.OnActorBeginOverlap`
  (params (OverlappedActor :type "Actor Object Reference") (OtherActor :type "Actor Object Reference"))
  (set `self.QueueLocation2Occupied` true)
  (goto _label))

(event `self.QueueLocation2.OnActorEndOverlap`
  (params (OverlappedActor :type "Actor Object Reference") (OtherActor :type "Actor Object Reference"))
  (set `self.QueueLocation2Occupied` false)
  (goto _label_2))

(event `self.QueueLocation3.OnActorBeginOverlap`
  (params (OverlappedActor :type "Actor Object Reference") (OtherActor :type "Actor Object Reference"))
  (set `self.QueueLocation3Occupied` true)
  (goto _label))

(event `self.QueueLocation3.OnActorEndOverlap`
  (params (OverlappedActor :type "Actor Object Reference") (OtherActor :type "Actor Object Reference"))
  (set `self.QueueLocation3Occupied` false)
  (goto _label_2))

(fn `GetNextFreeQueueLocation`
  (returns (FreeLocationTargetPoint :type "TargetPoint Object Reference"))
  (locals (NextFreeTargetLocation :type "TargetPoint Object Reference"))
  ;[1 1 1] Function assumes caller to first check if IsQueueFull = false. Afterwards check if targetpoint1 is occupied, if yes, check targetpoint2, if yes, return targetpoint3
  (if (`self.QueueLocation1Occupied`)
    (if (`self.QueueLocation2Occupied`)
      (set `local.NextFreeTargetLocation` (`self.QueueLocation3`))
      (else
        (set `local.NextFreeTargetLocation` (`self.QueueLocation2`))))
    (else
      (set `local.NextFreeTargetLocation` (`self.QueueLocation1CheckOut`))))
  (return (`local.NextFreeTargetLocation`)))

(fn `UserConstructionScript`)