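; Traffic light actor for the map that cycles its paired lamps on a timer and stops or releases vehicles.
; A looping FlipFlop, seeded by StartRed, alternates red and green with orange between each, holding red for an extra delay.
; Each switch function sets lamp visibility and CanDriveThrough.
; Overlapping BP_Vehicle_Master cars drive or stop on that flag, rechecked through one RetriggerableDelay, so only the latest car is polled.
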(event `self.ReceiveBeginPlay`
  (bind _startred (`self.StartRed`))
  (if _startred
    ;[1 1 1] initiation
    (`self.SwitchToRed`)
    (else
      (`self.SwitchToGreen`)))
  ;[1 1 1] Logic for timed traffic lights
  (`KismetSystemLibrary.Delay` 10.0 :!label _label)
  (`self.SwitchToOrange`)
  (`KismetSystemLibrary.Delay` 2.0)
  (if _startred
    (`/Engine/EditorBlueprintResources/StandardMacros.FlipFlop`
      (:`A`
        _)
      (:`B`
        (`self.SwitchToRed` :!label _label_2)
        (`KismetSystemLibrary.Delay` 10.0)
        (goto _label)))
    (else
      (`/Engine/EditorBlueprintResources/StandardMacros.FlipFlop`
        (:`A`
          (goto _label_2))
        (:`B`
          _))))
  (`self.SwitchToGreen`)
  (goto _label))

(event `self.CollisionBox.OnComponentBeginOverlap`
  (params (OverlappedComponent :type "PrimitiveComponent Object Reference") (OtherActor :type "Actor Object Reference") (OtherComp :type "PrimitiveComponent Object Reference") (OtherBodyIndex :type Integer) (bFromSweep :type Boolean) (SweepResult :type "HitResult Structure (by ref)"))
  ;[1 1 1] Logic when cars are in front of traffic light
  (bind _asbp_vehicle_master (cast `/Game/NPC/Vehicles/BP_Vehicle_Master` OtherActor))
  (if (`self.CanDriveThrough`) :!label _label_3
    (`/Game/NPC/Vehicles/BP_Vehicle_Master.Drive` _asbp_vehicle_master)
    (else
      (`/Game/NPC/Vehicles/BP_Vehicle_Master.Stop` _asbp_vehicle_master)
      (`KismetSystemLibrary.RetriggerableDelay` 1.0) ; Check the status of the light every 1 second when stopped
      (goto _label_3))))

(fn `SwitchToGreen`
  (set `self.CanDriveThrough` true) ; If red/orange,  status = false, if green, status = true
  (`|ExecutionSequence`
    (:`then_0`
      (`SceneComponent.SetHiddenInGame` (`self.GreenLight1`) false false)
      (`SceneComponent.SetHiddenInGame` (`self.GreenLight2`) false false))
    (:`then_1`
      (`SceneComponent.SetHiddenInGame` (`self.RedLight1`) true false)
      (`SceneComponent.SetHiddenInGame` (`self.RedLight2`) true false)
      (`SceneComponent.SetHiddenInGame` (`self.OrangeLight1`) true false)
      (`SceneComponent.SetHiddenInGame` (`self.OrangeLight2`) true false))))

(fn `SwitchToOrange`
  (set `self.CanDriveThrough` false) ; If red/orange,  status = false, if green, status = true
  (`|ExecutionSequence`
    (:`then_0`
      (`SceneComponent.SetHiddenInGame` (`self.OrangeLight1`) false false)
      (`SceneComponent.SetHiddenInGame` (`self.OrangeLight2`) false false))
    (:`then_1`
      (`SceneComponent.SetHiddenInGame` (`self.RedLight1`) true false)
      (`SceneComponent.SetHiddenInGame` (`self.RedLight2`) true false)
      (`SceneComponent.SetHiddenInGame` (`self.GreenLight1`) true false)
      (`SceneComponent.SetHiddenInGame` (`self.GreenLight2`) true false))))

(fn `SwitchToRed`
  (set `self.CanDriveThrough` false) ; If red/orange,  status = false, if green, status = true
  (`|ExecutionSequence`
    (:`then_0`
      (`SceneComponent.SetHiddenInGame` (`self.RedLight1`) false false)
      (`SceneComponent.SetHiddenInGame` (`self.RedLight2`) false false))
    (:`then_1`
      (`SceneComponent.SetHiddenInGame` (`self.GreenLight1`) true false)
      (`SceneComponent.SetHiddenInGame` (`self.GreenLight2`) true false)
      (`SceneComponent.SetHiddenInGame` (`self.OrangeLight1`) true false)
      (`SceneComponent.SetHiddenInGame` (`self.OrangeLight2`) true false))))

(fn `UserConstructionScript`)