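; Master Blueprint for AI traffic cars that drive along road splines and steer into parking spots.
; Tick steers toward a look-ahead point on the current path or parking spline, stopping once parked.
; A front collision box stops the car for actors other than roads, parking and traffic lights, resuming after a delay; Stop and Drive toggle brake lights.
; Spawn randomizes body color and sets destination; speed-limit regulation and pawn sensing are disconnected.
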(event `self.ReceiveTick`
  (params (DeltaSeconds :type "Float (single-precision)"))
  (bind _vehiclemovementcomponent (`self.VehicleMovementComponent`))
  ;[1 1 1] Steering / turn logic - based on following a spline
  (if (`self.hasFoundParkingSpot`)
    (if (`self.isParked`)
      (`self.Stop`)
      (else
        (bind _steering (`self.GetDirectionsBasedOnSpline` (`self.ParkingSteeringPosition`))) ; Is driving to parking spot
        (`ChaosVehicleMovementComponent.SetSteeringInput` _vehiclemovementcomponent _steering)))
    (else
      (bind _steering_2 (`self.GetDirectionsBasedOnSpline` (`self.CurrentPath`)))
      (`ChaosVehicleMovementComponent.SetSteeringInput` _vehiclemovementcomponent _steering_2)
      ;[1 1 1] debugging using a text element on top of the car
      (`TextRenderComponent.K2_SetText` (`self.TextRender`) (`KismetTextLibrary.Conv_DoubleToText` (* (`ChaosVehicleMovementComponent.GetForwardSpeed` (`self.VehicleMovementComponent`)) 0.036) "HalfToEven")))))

(event `self.ReceiveBeginPlay`
  ;[1 1 1] Movement control - drive or stop/wait logic
  (`self.Spawn`))

(event `self.CollisionBoxFront.OnComponentBeginOverlap`
  (params (OverlappedComponent :type "PrimitiveComponent Object Reference") (OtherActor :type "Actor Object Reference") (OtherComp :type "PrimitiveComponent Object Reference") (OtherBodyIndex :type Integer) (bFromSweep :type Boolean) (SweepResult :type "HitResult Structure (by ref)"))
  ;[1 1 1] Movement control - drive or stop/wait logic
  ;;[1 1 1] Have car stop when something is overlapping with the front collision box
  (cast `/Game/Maps/Blueprints/Actor/InvisibleMapLogic/BP_ParkingSpot` OtherActor ; Cast to parking spot to check if the actor it collided with\nis of class parking spot, because get class and "if class = parking spot" \nlogic does not exist in UE. If the cast fails, it means this actor is NOT a\nparking spot. On parking spot collission, the car should not stop but\ninstead follow the logic in the BP_Parkingspot blueprint.
    (:`CastFailed`
      (cast `/Game/Maps/Blueprints/Actor/InvisibleMapLogic/BP_RoadPiece3LanesWithNav` OtherActor
        (:`CastFailed`
          (cast `/Game/Maps/Blueprints/Actor/InvisibleMapLogic/BP_RoadPiece3Lanes1BusLaneWithNav` OtherActor
            (:`CastFailed`
              (cast `/Game/Maps/Blueprints/Actor/InvisibleMapLogic/BP_RoadPieceCrossroadWithNav` OtherActor
                (:`CastFailed`
                  (cast `/Game/Maps/Blueprints/Actor/InvisibleMapLogic/BP_RoadPieceCrossroadParkingWithNav` OtherActor
                    (:`CastFailed`
                      (cast `/Game/Maps/Blueprints/Actor/InvisibleMapLogic/BP_ParkingLot` OtherActor
                        (:`CastFailed`
                          (cast `/Game/Maps/Blueprints/Actor/InteractiveMapElements/BP_TrafficLights` OtherActor ; stop logic is in traffic lights itself, not here
                            (:`CastFailed`
                              (`self.Stop`))))))))))))))))

(event `self.PawnSensing.OnSeePawn`
  (params (Pawn :type "Pawn Object Reference"))
  ;[1 1 1] Movement control - drive or stop/wait logic
  ;;[1 1 1] Alternative way to stop the car when it sees something - DISABLED by removing line between On See Pawn and sequence block
)

(event `self.CollisionBoxFront.OnComponentEndOverlap`
  (params (OverlappedComponent :type "PrimitiveComponent Object Reference") (OtherActor :type "Actor Object Reference") (OtherComp :type "PrimitiveComponent Object Reference") (OtherBodyIndex :type Integer))
  ;[1 1 1] Movement control - drive or stop/wait logic
  ;;[1 1 1] Have car stop when something is overlapping with the front collision box
  (`KismetSystemLibrary.RetriggerableDelay` 2.0)
  (`self.Drive`))

(event `SpeedLimitChange`
  ;[1 1 1] Set speed
  ;;[1 1 1] temp disconnected
)

(fn `BrakeLights`
  (params (BrakeLights :type Boolean))
  (bind _returnvalue (`KismetMaterialLibrary.CreateDynamicMaterialInstance` "/Game/OtherUETemplates/Vehicles/SportsCar/Materials/MI_SportsCar_Chassis.MI_SportsCar_Chassis" "None"))
  (`PrimitiveComponent.SetMaterial` (`self.Mesh`) 1 _returnvalue)
  (if BrakeLights
    (`MaterialInstanceDynamic.SetScalarParameterValue` _returnvalue "BrakeLightPower" 200.0)
    (else
      (`MaterialInstanceDynamic.SetScalarParameterValue` _returnvalue "BrakeLightPower" 4.0))))

(fn `Drive`
  (bind _vehiclemovementcomponent (`self.VehicleMovementComponent`))
  (bind _output_get (set `self.CarStandsStill` false))
  (`ChaosVehicleMovementComponent.SetHandbrakeInput` _vehiclemovementcomponent _output_get)
  (`ChaosVehicleMovementComponent.SetThrottleInput` _vehiclemovementcomponent (`self.MaxSpeed`))
  (`self.BrakeLights` false))

(fn `GetDirectionsBasedOnSpline`
  (params (Spline :type "SplineComponent Object Reference"))
  (returns (Steering :type "Float (double-precision)"))
  (bind _returnvalue (`self.K2_GetActorLocation`))
  (bind (_returnvalue_roll _returnvalue_pitch _returnvalue_yaw) (`KismetMathLibrary.BreakRotator` (`KismetMathLibrary.NormalizedDeltaRotator` (`KismetMathLibrary.FindLookAtRotation` _returnvalue (`SplineComponent.FindLocationClosestToWorldLocation` Spline (+ (* (`KismetMathLibrary.Normal` (`SplineComponent.FindTangentClosestToWorldLocation` Spline _returnvalue "World")) 500.0) _returnvalue) "World")) (`self.K2_GetActorRotation`))))
  (`/Engine/EditorBlueprintResources/StandardMacros.IsValid` Spline
    (:`Is Valid`
      (return (`KismetMathLibrary.MapRangeClamped` _returnvalue_yaw -90.0 90.0 -1.0 1.0)))))

(fn `SetMaxSpeedToDefaultMaxSpeed`
  (set `self.MaxSpeed` (`self.Maximum Speed Default`)))

(fn `Spawn`
  ;[1 1 1] set random car body color
  (`PrimitiveComponent.SetMaterial` (`self.Mesh`) 0 (`|GetArrayItem` (`self.PossibleBodyColors`) (`KismetMathLibrary.RandomIntegerInRange` 0 4))) ; In slot 0 - the carbody texture should be. Here we set it\nto the colortexture stored in the array of possible\ncolors on index = randomintegerinrange
  ;[1 1 1] set random destination
  (bind _output_get (set `self.CurrentDestination` (cast `/Game/NPC/Vehicles/VehicleDestinations` (`KismetMathLibrary.Conv_IntToByte` (`KismetMathLibrary.RandomIntegerInRange` 0)))))
  (switch `/Game/NPC/Vehicles/VehicleDestinations` _output_get ; if parking lot or warehouse loading docks as destination - set "isgoingtopark" boolean
    (:`NewEnumerator0`
      (set `self.isGoingToPark` false :!label _label))
    (:`NewEnumerator1`
      (goto _label))
    (:`NewEnumerator2`
      _)
    (:`NewEnumerator3`
      _)
    (:`NewEnumerator4`
      _))
  (`self.SetMaxSpeedToDefaultMaxSpeed`)
  (`self.Drive`)
  (set `self.isParked` false))

(fn `Stop`
  (bind _vehiclemovementcomponent (`self.VehicleMovementComponent`))
  (`ChaosVehicleMovementComponent.SetThrottleInput` _vehiclemovementcomponent 0.0)
  (set `self.CarStandsStill` true)
  (`ChaosVehicleMovementComponent.SetHandbrakeInput` _vehiclemovementcomponent (`self.CarStandsStill`))
  (`self.BrakeLights` true))

(fn `UserConstructionScript`
  (set `self.Maximum Speed Default` 0.1) ; if car spawned by code later in the game\nand not at "beginplay" by putting the car into the map
  (`self.Spawn`))