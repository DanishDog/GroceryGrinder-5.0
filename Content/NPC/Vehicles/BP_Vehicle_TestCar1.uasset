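; An AI test car that drives itself along the first BP_DrivingPath spline found in the level.
; Each tick it steers toward the closest spline point to a spot projected ahead along the path tangent, mapping yaw difference to steering.
; BeginPlay applies throttle and dims brake lights through a dynamic material.
; Seeing a pawn cuts throttle and applies the handbrake, then a retriggerable five-second delay resumes driving.
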(event `self.ReceiveTick`
  (params (DeltaSeconds :type "Float (single-precision)"))
  ;[1 1 1] Steering / turn logic
  (bind _outactors (`GameplayStatics.GetAllActorsOfClass` "/Game/Maps/Blueprints/Actor/InvisibleMapLogic/BP_DrivingPath.BP_DrivingPath_C"))
  (bind _steering (`self.GetPath` _outactors))
  (`ChaosVehicleMovementComponent.SetSteeringInput` (`self.VehicleMovementComponent`) _steering))

(event `self.ReceiveBeginPlay`
  (bind _vehiclemovementcomponent (`self.VehicleMovementComponent`))
  (bind _vehiclemovementcomponent_2 (`self.VehicleMovementComponent`))
  ;[1 1 1] Movement control
  ;;[1 1 1] Move Forward logic
  (if true
    (`ChaosVehicleMovementComponent.SetThrottleInput` _vehiclemovementcomponent (`self.Speed`)) ; Throttle = 1 = full speed
    (`ChaosVehicleMovementComponent.SetBrakeInput` _vehiclemovementcomponent 0.0)
    (`/Engine/EditorBlueprintResources/StandardMacros.DoOnce` false :!label _label
      (:`Completed`
        (`self.BrakeLights` false)))
    (else
      (`ChaosVehicleMovementComponent.SetBrakeInput` _vehiclemovementcomponent_2 0.0)
      (`ChaosVehicleMovementComponent.SetThrottleInput` _vehiclemovementcomponent_2 0.0)
      (`self.BrakeLights` true)
      (goto _label :!via `Reset`))))

(event `self.PawnSensing.OnSeePawn`
  (params (Pawn :type "Pawn Object Reference"))
  (`|ExecutionSequence`
    (:`then_0`
      (`self.Stop`))
    (:`then_1`
      (`KismetSystemLibrary.RetriggerableDelay` 5.0)
      (`self.Drive`))))

(fn `BrakeLights`
  (params (BrakeLights :type Boolean))
  (bind _returnvalue (`KismetMaterialLibrary.CreateDynamicMaterialInstance` "/Game/OtherUETemplates/Vehicles/SportsCar/Materials/MI_SportsCar_Chassis.MI_SportsCar_Chassis" "None"))
  (`PrimitiveComponent.SetMaterial` (`self.Mesh`) 1 _returnvalue)
  (if BrakeLights
    (`MaterialInstanceDynamic.SetScalarParameterValue` _returnvalue "BrakeLightPower" 200.0)
    (else
      (`MaterialInstanceDynamic.SetScalarParameterValue` _returnvalue "BrakeLightPower" 4.0))))

(fn `Drive`
  (bind _vehiclemovementcomponent (`self.VehicleMovementComponent`))
  (bind _output_get (set `self.CarStandsStill` false))
  (`ChaosVehicleMovementComponent.SetHandbrakeInput` _vehiclemovementcomponent _output_get)
  (`ChaosVehicleMovementComponent.SetThrottleInput` _vehiclemovementcomponent (`self.Speed`)))

(fn `GetPath`
  (params (Splines :type "Array of /Game/Maps/Blueprints/Actor/InvisibleMapLogic/BP_DrivingPath Object Reference"))
  (returns (Steering :type "Float (double-precision)"))
  (bind _returnvalue (`self.K2_GetActorLocation`))
  (bind _spline (`/Game/Maps/Blueprints/Actor/InvisibleMapLogic/BP_DrivingPath.Spline` (`|GetArrayItem` Splines)))
  (bind (_returnvalue_roll _returnvalue_pitch _returnvalue_yaw) (`KismetMathLibrary.BreakRotator` (`KismetMathLibrary.NormalizedDeltaRotator` (`KismetMathLibrary.FindLookAtRotation` _returnvalue (`SplineComponent.FindLocationClosestToWorldLocation` _spline (+ (* (`KismetMathLibrary.Normal` (`SplineComponent.FindTangentClosestToWorldLocation` _spline _returnvalue "Local")) 500.0) _returnvalue) "World")) (`self.K2_GetActorRotation`))))
  (return (`KismetMathLibrary.MapRangeClamped` _returnvalue_yaw -90.0 90.0 -1.0 1.0)))

(fn `Stop`
  (bind _vehiclemovementcomponent (`self.VehicleMovementComponent`))
  (`ChaosVehicleMovementComponent.SetThrottleInput` _vehiclemovementcomponent 0.0)
  (set `self.CarStandsStill` true)
  (`ChaosVehicleMovementComponent.SetHandbrakeInput` _vehiclemovementcomponent (`self.CarStandsStill`)))

(fn `UserConstructionScript`)