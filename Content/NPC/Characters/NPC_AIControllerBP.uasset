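; AI controller for NPC characters that runs a behavior tree and reacts to perceiving the player.
; The NPC passes its behavior tree into SetupAIController, which starts it and sets the default patrol path direction in the Blackboard.
; AI perception updates cast the sensed actor to ThirdPersonCharacter and write the sensing result to the CanSeePlayer key.
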(event `Setup AIController`
  (params (BehaviorTree :type "BehaviorTree Object Reference"))
  (set `self.BehaviorTree` BehaviorTree) ; Link the behavior tree for the character to the AIcontroller class.\nWe get the correct value for the behavior tree by getting it as input \nwhen launching the Setup AIController event from within the Event Graph\nof the NPCCharacter.
  (`self.RunBehaviorTree` (`self.BehaviorTree`))
  ;[1 1 1] Default blackboard key values
  (`BlackboardComponent.SetValueAsBool` (`self.Blackboard`) "PatrollingPathDirection" true))

(event `self.ReceiveBeginPlay`)

(event `self.AIPerception.OnTargetPerceptionUpdated`
  (params (Actor :type "Actor Object Reference") (Stimulus :type "AIStimulus Structure"))
  ;[1 1 1] Based on the guard character seeing the player character (= one of the stimuli sources for AIPerception), set the blackoard key to true
  (cast `/Game/ThirdPersonBP/Blueprints/ThirdPersonCharacter` Actor) ; If the cast works, we will set the blackboard value "can see player". If fails, it was not the player it saw.
  (`BlackboardComponent.SetValueAsBool` (`self.Blackboard`) "CanSeePlayer" (`.bSuccessfullySensed` (break `AIStimulus` Stimulus))))

(fn `UserConstructionScript`)